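; BP_NapkinSpawner is a collectible spawner actor that places one napkin pickup at a randomly chosen location in the level.
; On BeginPlay it picks one of three NapkinOnLocation components at random and stores that component's world position.
; It then spawns the CollectNapkin class at that position, so the napkin's placement can differ each play session.
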(event `self.ReceiveBeginPlay`
  (switch `int` (`KismetMathLibrary.RandomIntegerInRange` 0 2)
    (:`0`
      (set `self.NapkinLocationSpawner` (`SceneComponent.K2_GetComponentLocation` (`self.NapkinOnLocation`))))
    (:`1`
      (set `self.NapkinLocationSpawner` (`SceneComponent.K2_GetComponentLocation` (`self.NapkinOnLocation1`))))
    (:`2`
      (set `self.NapkinLocationSpawner` (`SceneComponent.K2_GetComponentLocation` (`self.NapkinOnLocation2`)))))
  (`|SpawnActorFromClass` "/Game/Collectibles/CollectibleActors/CollectNapkin.CollectNapkin_C" (`KismetMathLibrary.Conv_VectorToTransform` (`self.NapkinLocationSpawner`)) "Undefined" "MultiplyWithRoot" null null))

(fn `UserConstructionScript`)