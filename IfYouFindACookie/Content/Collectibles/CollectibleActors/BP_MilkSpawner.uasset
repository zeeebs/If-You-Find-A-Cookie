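; BP_MilkSpawner is a spawner actor that places a CollectMilk collectible at a randomly picked spot when play begins.
; A random switch with three cases copies the world location of a marker component into MilkLocationSpawner, which feeds a single shared SpawnActor call.
; Two of the cases read MilkOnLocation1 and one reads MilkOnLocation, so only two spots are possible and MilkOnLocation1 is twice as likely.
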(event `self.ReceiveBeginPlay`
  (switch `int` (`KismetMathLibrary.RandomIntegerInRange` 0 2)
    (:`0`
      (set `self.MilkLocationSpawner` (`SceneComponent.K2_GetComponentLocation` (`self.MilkOnLocation1`))))
    (:`1`
      (set `self.MilkLocationSpawner` (`SceneComponent.K2_GetComponentLocation` (`self.MilkOnLocation1`))))
    (:`2`
      (set `self.MilkLocationSpawner` (`SceneComponent.K2_GetComponentLocation` (`self.MilkOnLocation`)))))
  (`|SpawnActorFromClass` "/Game/Collectibles/CollectibleActors/CollectMilk.CollectMilk_C" (`KismetMathLibrary.Conv_VectorToTransform` (`self.MilkLocationSpawner`)) "Undefined" "MultiplyWithRoot" null null))

(fn `UserConstructionScript`)