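; BP_CookieSpawner is an actor that spawns one collectible cookie at a randomly chosen spot when play begins.
; BeginPlay picks one of three placed location components at random and stores its world location in CookieSpawnLocation.
; It then spawns a CollectCookie actor at that location through a single shared spawn node.
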(event `self.ReceiveBeginPlay`
  (switch `int` (`KismetMathLibrary.RandomIntegerInRange` 0 2)
    (:`0`
      (set `self.CookieSpawnLocation` (`SceneComponent.K2_GetComponentLocation` (`self.CookieOnLocation`))))
    (:`1`
      (set `self.CookieSpawnLocation` (`SceneComponent.K2_GetComponentLocation` (`self.CookieOnLocation1`))))
    (:`2`
      (set `self.CookieSpawnLocation` (`SceneComponent.K2_GetComponentLocation` (`self.CookieOnLocation2`)))))
  (`|SpawnActorFromClass` "/Game/Collectibles/CollectibleActors/CollectCookie.CollectCookie_C" (`KismetMathLibrary.Conv_VectorToTransform` (`self.CookieSpawnLocation`)) "Undefined" "MultiplyWithRoot" null null))

(fn `UserConstructionScript`)