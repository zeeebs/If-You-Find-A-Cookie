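; BP_CupSpawner is a collectible spawner actor that places a CollectCup at one of three possible spots.
; On BeginPlay it picks a random index and takes the world location of the matching CupOnLocation component.
; All three branches share a single SpawnActor call, which uses only that location for the spawn transform.
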(event `self.ReceiveBeginPlay`
  (switch `int` (`KismetMathLibrary.RandomIntegerInRange` 0 2)
    (:`0`
      (set `self.CupSpawnLocation` (`SceneComponent.K2_GetComponentLocation` (`self.CupOnLocation`))))
    (:`1`
      (set `self.CupSpawnLocation` (`SceneComponent.K2_GetComponentLocation` (`self.CupOnLocation1`))))
    (:`2`
      (set `self.CupSpawnLocation` (`SceneComponent.K2_GetComponentLocation` (`self.CupOnLocation2`)))))
  (`|SpawnActorFromClass` "/Game/Collectibles/CollectibleActors/CollectCup.CollectCup_C" (`KismetMathLibrary.Conv_VectorToTransform` (`self.CupSpawnLocation`)) "Undefined" "MultiplyWithRoot" null null))

(fn `UserConstructionScript`)