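; Collectible spawner actor that places a CollectPlate at one of three preset locations when play begins.
; BeginPlay picks a random index from 0 to 2 and stores the world location of the matching PlateOnLocation component.
; All three branches feed a single spawn call, which creates the plate at that stored location.
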(event `self.ReceiveBeginPlay`
  (switch `int` (`KismetMathLibrary.RandomIntegerInRange` 0 2)
    (:`0`
      (set `self.PlateLocationSpawner` (`SceneComponent.K2_GetComponentLocation` (`self.PlateOnLocation`))))
    (:`1`
      (set `self.PlateLocationSpawner` (`SceneComponent.K2_GetComponentLocation` (`self.PlateOnLocation1`))))
    (:`2`
      (set `self.PlateLocationSpawner` (`SceneComponent.K2_GetComponentLocation` (`self.PlateOnLocation2`)))))
  (`|SpawnActorFromClass` "/Game/Collectibles/CollectibleActors/CollectPlate.CollectPlate_C" (`KismetMathLibrary.Conv_VectorToTransform` (`self.PlateLocationSpawner`)) "Undefined" "MultiplyWithRoot" null null))

(fn `UserConstructionScript`)